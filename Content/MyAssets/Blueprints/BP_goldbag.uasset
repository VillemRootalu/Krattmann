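; Gold bag pickup that a BP_Player_Test collects by overlapping it.
; On overlap it plays a gold sound at the world origin, hides itself, disables the mesh's collision and calls UpdateGoldbags on the player.
; After a random delay it respawns in place by unhiding and restoring collision, so the actor is reused rather than destroyed.
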(event `self.ReceiveActorBeginOverlap`
  (params (OtherActor :type "Actor Object Reference"))
  (bind _asbp_player_test (cast `/Game/MyAssets/Blueprints/BP_Player_Test` OtherActor))
  (`GameplayStatics.PlaySoundAtLocation` "/Game/Audio/SFX/SFX_Gold_Cue.SFX_Gold_Cue" (0.0 0.0 0.0) (struct) 1.0 1.0 0.0 null null null)
  ;[1 1 1] Despawn
  (`SceneComponent.SetHiddenInGame` (`self.DefaultSceneRoot`) true true)
  (`PrimitiveComponent.SetCollisionEnabled` (`self.StaticMesh_goldbag`) "NoCollision")
  ;[1 1 1] Set Gold
  (`/Game/MyAssets/Blueprints/BP_Player_Test.Update_goldbags` _asbp_player_test)
  ;[1 1 1] Random Delay
  (`KismetSystemLibrary.Delay` (`KismetMathLibrary.RandomFloatInRange` 10.0 30.0))
  ;[1 1 1] Respawn
  (`SceneComponent.SetHiddenInGame` (`self.DefaultSceneRoot`) false true)
  (`PrimitiveComponent.SetCollisionEnabled` (`self.StaticMesh_goldbag`) "QueryAndPhysics"))

(fn `UserConstructionScript`)